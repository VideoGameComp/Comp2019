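; Goblin enemy with a flipbook sprite that chases the player on the X/Z plane and attacks on contact.
; Tick adds movement toward the player beyond a set distance and picks directional idle or move flipbooks, marked as not working.
; Capsule overlap starts a delay-based loop that damages the player while in range, briefly locking orientation for a single attack flipbook.
; A directional attack variant remains unconnected.
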(event `self.ReceiveBeginPlay`
  ;[1 1 1] Goblin Speed
  (set `CharacterMovementComponent.MaxFlySpeed` (`self.Speed`) (`self.CharacterMovement`)))

(event `self.ReceiveTick`
  (params (DeltaSeconds :type "Float (single-precision)"))
  (bind (_returnvalue_x _returnvalue_y _returnvalue_z) (`KismetMathLibrary.BreakVector` (`self.K2_GetActorLocation`)))
  (bind _distance (`self.Distance`))
  (bind (_returnvalue_x_2 _returnvalue_y_2 _returnvalue_z_2) (`KismetMathLibrary.BreakVector` (`self.K2_GetActorLocation` (`GameplayStatics.GetPlayerCharacter` 0))))
  (bind _returnvalue (- _returnvalue_x_2 _returnvalue_x))
  (bind _returnvalue_2 (- _returnvalue_z_2 _returnvalue_z))
  (`|ExecutionSequence`
    (:`then_0`
      ;[1 1 1] Following System
      (set `self.XDirection` _returnvalue)
      (set `self.ZDirection` _returnvalue_2)
      (if (or (>= (`KismetMathLibrary.Abs` _returnvalue) _distance) (>= (`KismetMathLibrary.Abs` _returnvalue_2) _distance))
        (`self.AddMovementInput` (`KismetMathLibrary.MakeVector` (`self.XDirection`) 0.0 (`self.ZDirection`)))))
    (:`then_1`
      ;[1 1 1] Refresh Goblin Orientation (not working)
      (if (`self.CanOrient`)
        (`self.GoblinOrientation`)))))

(event `self.CapsuleComponent.OnComponentBeginOverlap`
  (params (OverlappedComponent :type "PrimitiveComponent Object Reference") (OtherActor :type "Actor Object Reference") (OtherComp :type "PrimitiveComponent Object Reference") (OtherBodyIndex :type Integer) (bFromSweep :type Boolean) (SweepResult :type "HitResult Structure (by ref)"))
  ;[1 1 1] Attack System
  (bind _asplayer_bp (cast `/Game/Blueprints/Player/PlayerBP` OtherActor))
  (set `self.InRange` true)
  (if (`self.CanAttack`)
    (`KismetSystemLibrary.Delay` 0.2)
    (if (`self.InRange`) :!label _label
      (`PaperFlipbookComponent.SetFlipbook` (`self.Sprite`) "/Game/Assets/Goblin/GoblinFB/G-DAttack.G-DAttack")
      (set `self.CanAttack` false)
      (set `self.CanOrient` false)
      (`/Engine/EditorBlueprintResources/StandardMacros.DecrementInt` (`/Game/Blueprints/Player/PlayerBP.Health` _asplayer_bp)
        (:`  `
          (`/Game/Blueprints/Player/PlayerBP.Take Damage` _asplayer_bp)
          (`KismetSystemLibrary.Delay` 0.1)
          (set `self.CanOrient` true)
          (`KismetSystemLibrary.Delay` (`self.AttackSpeed`))
          (set `self.CanAttack` true)
          (goto _label))))))

(event `self.CapsuleComponent.OnComponentEndOverlap`
  (params (OverlappedComponent :type "PrimitiveComponent Object Reference") (OtherActor :type "Actor Object Reference") (OtherComp :type "PrimitiveComponent Object Reference") (OtherBodyIndex :type Integer))
  ;[1 1 1] Attack System
  (cast `/Game/Blueprints/Player/PlayerBP` OtherActor)
  (set `self.InRange` false))

(event `InputAction|Attack`
  (params (Key :type "Key Structure"))
  ;[1 1 1] Temporary Shit (could be useful)
)

(fn `GoblinOrientation`
  (bind (_movementlist_upidle _movementlist_downidle _movementlist_leftidle _movementlist_rightidle _movementlist_upmove _movementlist_downmove _movementlist_leftmove _movementlist_rightmove) (break `/Game/Blueprints/Goblin/GoblinStruct` (`self.MovementList`)))
  (bind _zdirection (`self.ZDirection`))
  (if (or (!= (`self.ZDirection`) 0.0) (!= (`self.XDirection`) 0.0))
    (bind _output_get (set `self.LastMovementDirection` (select `bool` (> _zdirection 0.0) :`false` (select `bool` (< _zdirection 0.0) :`false` (select `bool` (> (`self.XDirection`) 0.0) :`false` "NewEnumerator2" :`true` "NewEnumerator3" :!type "/Game/Blueprints/OrientationEnum Enum") :`true` "NewEnumerator1") :`true` "NewEnumerator0"))))
  (`PaperFlipbookComponent.SetFlipbook` (`self.Sprite`) (select `bool` (> (`KismetMathLibrary.VSize` (`self.GetVelocity`)) 0.0) :`false` (select `/Game/Blueprints/OrientationEnum` _output_get :`NewEnumerator0` _movementlist_upidle :`NewEnumerator1` _movementlist_downidle :`NewEnumerator2` _movementlist_leftidle :`NewEnumerator3` _movementlist_rightidle) :`true` (select `/Game/Blueprints/OrientationEnum` _output_get :`NewEnumerator0` _movementlist_upmove :`NewEnumerator1` _movementlist_downmove :`NewEnumerator2` _movementlist_leftmove :`NewEnumerator3` _movementlist_rightmove))))

(fn `UserConstructionScript`)