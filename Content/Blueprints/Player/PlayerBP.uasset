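; Player character for a 2D sprite goblin-slaying game, which also runs the game flow: menus, HUD, death, restart and saved scores.
; Axis input moves it four ways on the XZ plane, driving directional flipbooks.
; HitRange overlaps set the target for timed sword attacks, which add multiplier-scaled score, and grant health from beer pickups.
; Tick-driven Delays act as repeating timers for random goblin spawns and multiplier growth.
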(event `self.ReceiveBeginPlay`
  (bind _returnvalue (`GameplayStatics.GetPlayerController` 0))
  (bind _returnvalue_2 (`GameplayStatics.SpawnSound2D` "/Game/Sounds/Main_Menu_Cue.Main_Menu_Cue" 1.0 1.0 0.0 null))
  (set `self.InitialLocation` (`self.K2_GetActorLocation`))
  (`GameplayStatics.SetGamePaused` true)
  (bind _returnvalue_3 (`|CreateWidget` "/Game/Widget/MainMenu/Menu.Menu_C"))
  (`UserWidget.AddToViewport` _returnvalue_3 0)
  (`WidgetBlueprintLibrary.SetInputMode_GameAndUIEx` _returnvalue _returnvalue_3 "DoNotLock" false)
  (set `PlayerController.bShowMouseCursor` true _returnvalue))

(event `InitializeGame`
  (bind _returnvalue (`GameplayStatics.GetPlayerController` 0))
  ;[1 1 1] Create UI & Load Stats
  (`AudioComponent.Stop` (stale `self.ReceiveBeginPlay` _returnvalue_2))
  (`WidgetBlueprintLibrary.SetInputMode_GameOnly` _returnvalue)
  (set `PlayerController.bShowMouseCursor` false _returnvalue)
  (`Widget.RemoveFromParent` (stale `self.ReceiveBeginPlay` _returnvalue_3))
  (`GameplayStatics.SetGamePaused` false)
  (bind _returnvalue_2 (`|CreateWidget` "/Game/Widget/InGame/PlayerUI.PlayerUI_C"))
  (bind _output_get (set `self.PlayerUIRef` _returnvalue_2))
  (`UserWidget.AddToViewport` _output_get 0)
  (`self.Load - SaveGame`)
  (`self.ResetValues`)
  (`GameplayStatics.SpawnSound2D` "/Game/Sounds/BGM-1_Cue.BGM-1_Cue" 1.0 1.0 0.0 null))

(event `InputAction|Quit`
  (params (Key :type "Key Structure"))
  (:`Pressed`
    (`KismetSystemLibrary.ExecuteConsoleCommand` "quit" null)))

(event `Death`
  (bind _returnvalue (`GameplayStatics.GetPlayerController` 0))
  ;[1 1 1] Death
  (`GameplayStatics.SetGamePaused` true)
  (`self.Save - SaveGame`)
  (bind _returnvalue_2 (`|CreateWidget` "/Game/Widget/Score/ScoreMenu.ScoreMenu_C"))
  (`UserWidget.AddToViewport` _returnvalue_2 0)
  (`WidgetBlueprintLibrary.SetInputMode_GameAndUIEx` _returnvalue _returnvalue_2 "DoNotLock" false)
  (set `PlayerController.bShowMouseCursor` true _returnvalue))

(event `InputAxis|Up/Down`
  (params (AxisValue :type "Float (single-precision)"))
  ;[1 1 1] Movement
  (if (== (`self.GetInputAxisValue`) 0.0)
    (`self.AddMovementInput` (0.0 0.0 1.0) AxisValue)))

(event `ResetValues`
  ;[1 1 1] ResetValues
  (`|ExecutionSequence`
    (:`then_0`
      (set `self.Multiplier` 1.0)
      (set `self.Health` 3)
      (set `self.NewScore` 0)
      (set `self.AttackSpeed` 0.2))
    (:`then_1`
      (set `self.SpawnTime` 5.0)
      (set `self.SpawnNumber` 1.0))))

(event `ReloadGame`
  (bind _returnvalue (`GameplayStatics.GetPlayerController` 0))
  (`GameplayStatics.SetGamePaused` false)
  ;[1 1 1] Create UI & Load Stats
  (`WidgetBlueprintLibrary.SetInputMode_GameOnly` _returnvalue)
  (set `PlayerController.bShowMouseCursor` false _returnvalue)
  (`Widget.RemoveFromParent` (stale `Death` _returnvalue_2))
  (bind _returnvalue_2 (`|CreateWidget` "/Game/Widget/InGame/PlayerUI.PlayerUI_C"))
  (bind _output_get (set `self.PlayerUIRef` _returnvalue_2))
  (`UserWidget.AddToViewport` _output_get 0)
  (bind _outactors (`GameplayStatics.GetAllActorsOfClass` "/Game/Blueprints/Goblin/GoblinBP.GoblinBP_C"))
  (`self.K2_DestroyActor` _outactors)
  (`self.Load - SaveGame`)
  (`self.ResetValues`)
  (`self.K2_TeleportTo` (`self.InitialLocation`)))

(event `InputAxis|Left/Right`
  (params (AxisValue :type "Float (single-precision)"))
  ;[1 1 1] Movement
  (if (== (`self.GetInputAxisValue`) 0.0)
    (`self.AddMovementInput` (1.0 0.0 0.0) AxisValue)))

(event `SwordSound`
  (`GameplayStatics.SpawnSound2D` "/Game/Sounds/Sword_SFX-1_Cue.Sword_SFX-1_Cue" 1.0 1.0 0.0 null))

(event `self.ReceiveTick`
  (params (DeltaSeconds :type "Float (single-precision)"))
  ;[1 1 1] Refresh Player Orientation
  (`|ExecutionSequence`
    (:`then_0`
      (if (`self.CanOrient`)
        (`self.PlayerOrientation`)))
    (:`then_1`
      (`KismetSystemLibrary.Delay` (`self.SpawnTime`))
      (`self.SpawnNew`))
    (:`then_2`
      ;[1 1 1] Update Multiplier
      (`KismetSystemLibrary.Delay` 10.0)
      (set `self.Multiplier` (* 1.5 (`self.Multiplier`))))))

(event `self.ReceiveAnyDamage`
  (params (Damage :type "Float (single-precision)") (DamageType :type "DamageType Object Reference") (InstigatedBy :type "Controller Object Reference") (DamageCauser :type "Actor Object Reference"))
  ;[1 1 1] Take Damage
  (`/Engine/EditorBlueprintResources/StandardMacros.DecrementInt` (`self.Health`)
    (:`  `
      (`GameplayStatics.PlayWorldCameraShake` "/Game/Blueprints/Player/PlayerShake.PlayerShake_C" (`self.K2_GetActorLocation`) 0.0 500.0)
      (if (<= (`self.Health`) 0)
        (`self.Death`)))))

(event `SpawnNew`
  (bind _returnvalue (`KismetMathLibrary.RandomFloatInRange` -512.0 512.0))
  (bind _output_get (set `self.SpawnTime` (* (`KismetMathLibrary.Sqrt` (`self.SpawnTime`)) 2.0)))
  (`AIBlueprintHelperLibrary.SpawnAIFromClass` "/Game/Blueprints/Goblin/GoblinBP.GoblinBP_C" null (`KismetMathLibrary.MakeVector` _returnvalue -15.0 _returnvalue))
  (`KismetSystemLibrary.PrintString` (`KismetStringLibrary.Conv_DoubleToString` _output_get)))

(event `InputAction|Attack`
  (params (Key :type "Key Structure"))
  (bind (_movementlist_upidle _movementlist_downidle _movementlist_leftidle _movementlist_rightidle _movementlist_upmove _movementlist_downmove _movementlist_leftmove _movementlist_rightmove _movementlist_upattack _movementlist_downattack _movementlist_leftattack _movementlist_rightattack) (break `/Game/Blueprints/Player/PlayerStruct` (`self.MovementList`)))
  ;[1 1 1] Attack
  (:`Pressed`
    (if (`self.CanAttack`)
      (`PaperFlipbookComponent.SetFlipbook` (`self.Sprite`) (select `/Game/Blueprints/OrientationEnum` (`self.LastMovementDirection`) :`NewEnumerator0` _movementlist_upattack :`NewEnumerator1` _movementlist_downattack :`NewEnumerator2` _movementlist_leftattack :`NewEnumerator3` _movementlist_rightattack))
      (`self.SwordSound`)
      (set `self.CanAttack` false)
      (set `self.CanOrient` false)
      (if (`self.InRange`)
        (`GameplayStatics.ApplyDamage` (`self.OverlappedComponent`) 1.0)
        (`KismetSystemLibrary.Delay` 0.1)
        (set `self.NewScore` (+ (`self.NewScore`) (`KismetMathLibrary.Round` (`self.Multiplier`)))))
      (`KismetSystemLibrary.Delay` 0.333333)
      (set `self.CanOrient` true)
      (`KismetSystemLibrary.Delay` (`self.AttackSpeed`))
      (set `self.CanAttack` true))))

(event `self.HitRange.OnComponentBeginOverlap`
  (params (OverlappedComponent :type "PrimitiveComponent Object Reference") (OtherActor :type "Actor Object Reference") (OtherComp :type "PrimitiveComponent Object Reference") (OtherBodyIndex :type Integer) (bFromSweep :type Boolean) (SweepResult :type "HitResult Structure (by ref)"))
  (bind _health (`self.Health`))
  ;[1 1 1] Enemy in range
  (bind _output_get (set `self.OverlappedComponent` OtherActor))
  (if (`ActorComponent.ComponentHasTag` OtherComp "GDamage")
    (set `self.InRange` true)
    (elif (and (`ActorComponent.ComponentHasTag` OtherComp "Beer") (< _health 3) (`self.PowerUpUsable`))
      (bind _aspower_up (cast `/Game/Blueprints/PowerUp` _output_get))
      (`/Engine/EditorBlueprintResources/StandardMacros.IncrementInt` _health
        (:`  `
          (bind _beer (`/Game/Blueprints/PowerUp.Beer` _aspower_up))
          (`SceneComponent.ToggleVisibility` _beer false)
          (`KismetSystemLibrary.PrintString` "Hello")
          (set `self.PowerUpUsable` false)
          (`KismetSystemLibrary.Delay` 5.0)
          (`SceneComponent.ToggleVisibility` _beer false)
          (`KismetSystemLibrary.PrintString` "Hello")
          (set `self.PowerUpUsable` true))))))

(event `self.HitRange.OnComponentEndOverlap`
  (params (OverlappedComponent :type "PrimitiveComponent Object Reference") (OtherActor :type "Actor Object Reference") (OtherComp :type "PrimitiveComponent Object Reference") (OtherBodyIndex :type Integer))
  ;[1 1 1] Enemy in range
  (if (`ActorComponent.ComponentHasTag` OtherComp "GDamage")
    (set `self.InRange` false)))

(fn `Load - SaveGame`
  (bind _returnvalue (`GameplayStatics.LoadGameFromSlot` "GameStats"))
  (bind _asgame_stats (cast `/Game/Blueprints/GameStats` _returnvalue)
    (:`then`
      (bind _output_get (set `self.GameStatsRef` _asgame_stats)))
    (:`CastFailed`
      (bind _returnvalue_2 (`GameplayStatics.CreateSaveGameObject` "/Game/Blueprints/GameStats.GameStats_C"))
      (set `self.GameStatsRef` _returnvalue_2)))
  (set `self.HighScore` (`/Game/Blueprints/GameStats.HighScore` _output_get)))

(fn `PlayerOrientation`
  (bind _returnvalue (`self.GetInputAxisValue`))
  (bind (_movementlist_upidle _movementlist_downidle _movementlist_leftidle _movementlist_rightidle _movementlist_upmove _movementlist_downmove _movementlist_leftmove _movementlist_rightmove) (break `/Game/Blueprints/Player/PlayerStruct` (`self.MovementList`)))
  (if (or (!= (`self.GetInputAxisValue`) 0.0) (!= (`self.GetInputAxisValue`) 0.0))
    (bind _output_get (set `self.LastMovementDirection` (select `bool` (> _returnvalue 0.0) :`false` (select `bool` (< _returnvalue 0.0) :`false` (select `bool` (> (`self.GetInputAxisValue`) 0.0) :`false` "NewEnumerator2" :`true` "NewEnumerator3" :!type "/Game/Blueprints/OrientationEnum Enum") :`true` "NewEnumerator1") :`true` "NewEnumerator0"))))
  (`PaperFlipbookComponent.SetFlipbook` (`self.Sprite`) (select `bool` (> (`KismetMathLibrary.VSize` (`self.GetVelocity`)) 0.0) :`false` (select `/Game/Blueprints/OrientationEnum` _output_get :`NewEnumerator0` _movementlist_upidle :`NewEnumerator1` _movementlist_downidle :`NewEnumerator2` _movementlist_leftidle :`NewEnumerator3` _movementlist_rightidle) :`true` (select `/Game/Blueprints/OrientationEnum` _output_get :`NewEnumerator0` _movementlist_upmove :`NewEnumerator1` _movementlist_downmove :`NewEnumerator2` _movementlist_leftmove :`NewEnumerator3` _movementlist_rightmove))))

(fn `Save - SaveGame`
  (bind _gamestatsref (`self.GameStatsRef`))
  (if (> (`self.NewScore`) (`self.HighScore`))
    (set `/Game/Blueprints/GameStats.HighScore` (`self.NewScore`) _gamestatsref))
  (`KismetArrayLibrary.Array_Add` (`/Game/Blueprints/GameStats.PreviousScores` _gamestatsref) (`self.NewScore`))
  (`GameplayStatics.SaveGameToSlot` (`self.GameStatsRef`) "GameStats")
  (`self.Load - SaveGame`))

(fn `UserConstructionScript`)